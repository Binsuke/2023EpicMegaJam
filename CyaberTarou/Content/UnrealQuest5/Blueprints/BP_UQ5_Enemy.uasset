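; Enemy Blueprint for UnrealQuest5 that attacks, takes damage and dies, using the Gameplay Ability System.
; BeginPlay grants its abilities and creates a viewport HP bar, which Tick repositions to a world anchor.
; Damage updates the bar and triggers a hit-reaction ability by tag.
; Death ragdolls the mesh, then hides it with an effect, increments the player's kill count and calls the GameMode's enemy check.
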(event Custom|AbilityInitialize
  (for _array_element (Variables|Default|GetAbility%20Class)
    (GameplayAbilities|GiveAbility (Variables|Default|GetAbilitySystem) _array_element 0 -1)))

(event Custom|Attack
  ;[1 0 0 0.5] 攻撃
  (Abilities|TryActivateAbilitiesbyTag (Variables|Default|GetAbilitySystem) (GameplayTags|MakeLiteralGameplayTagContainer "(GameplayTags=((TagName=\"Ability.Attack.C\")))") true))

(event Custom|DownEffect
  (Utilities|FlowControl|Delay 0.8)
  (Rendering|SetVisibility (Variables|Character|GetMesh) false false)
  (Niagara|SpawnSystemAttached "/Game/MyFolder/Effect/DownEffect.DownEffect" (Variables|Character|GetMesh) "None" "0, 0, 0" "0, 0, 0" "SnapToTarget" false)
  (Actor|SetLifeSpan 3.0)
  (CallFunction|EnemyDestroyedCall)
  (CallFunction|WidgetDestoy))

(event Custom|GotParis
  (if (Variables|Default|GetGotParied)
    (Abilities|TryActivateAbilitiesbyTag (Variables|Default|GetAbilitySystem) (GameplayTags|MakeLiteralGameplayTagContainer "(GameplayTags=)") true)))

(event Custom|EnemyDestroyedCall
  (Utilities|FlowControl|DoOnce false
    (:Completed
      (bind _asbp_uq5_player (Utilities|Casting|CastToBP_UQ5_Player (Game|Player|GetPlayerPawn 0)))
      (Variables|/Game/UnrealQuest5/Blueprints/BP_UQ5_Player.BP_UQ5_Player_C|SetDestroyedCount _asbp_uq5_player (+ (Variables|/Game/UnrealQuest5/Blueprints/BP_UQ5_Player.BP_UQ5_Player_C|GetDestroyedCount _asbp_uq5_player) 1))
      (bind _asbp_uq5_game_mode (Utilities|Casting|CastToBP_UQ5_GameMode (Game|GetGameMode)))
      (Default|EnemyCheck _asbp_uq5_game_mode))))

(event Custom|Widget
  (bind _returnvalue (UserInterface|CreateWidget "/Game/MyFolder/Widget/WBP_WIDGET.WBP_WIDGET_C" 0 (Variables|Default|GetHealth)))
  (bind _output_get (Variables|Default|SetHPBar _returnvalue))
  (UserInterface|Viewport|AddtoViewport _output_get 0))

(event Custom|WidgetDestoy
  (if (<= (Variables|Default|GetHealth) 0.0)
    (Widget|RemovefromParent (Variables|Default|GetHPBar))))

(event Game|Damage|EventAnyDamage
  (params (Damage :type Float%20%28single-precision%29) (DamageType :type Damage%20Type%20Object%20Reference) (InstigatedBy :type Controller%20Object%20Reference) (DamageCauser :type Actor%20Object%20Reference))
  (bind _output_get (Variables|Default|SetHealth (- (Variables|Default|GetHealth) Damage)))
  (Default|OnTakeDamage (Variables|Default|GetHPBar) Damage)
  (if (> _output_get 0.0)
    ;[1 0 0 0.5] 攻撃
    (Abilities|TryActivateAbilitiesbyTag (Variables|Default|GetAbilitySystem) (GameplayTags|MakeLiteralGameplayTagContainer "(GameplayTags=((TagName=\"Ability.Damaged\")))") true)
    (else
      (Class|SkeletalMeshComponent|SetAllBodiesSimulatePhysics (Variables|Character|GetMesh) true)
      (Collision|SetCollisionEnabled (Variables|Character|GetMesh) "PhysicsOnly")
      (CallFunction|DownEffect))))

(event EventTick
  (params (DeltaSeconds :type Float%20%28single-precision%29))
  (bind _hpbar (Variables|Default|GetHPBar)
    (:then
      (Default|UpdateUILocation _hpbar (Transformation|GetWorldLocation (Variables|Default|GetUIPos))))
    (:else)))

(event EventBeginPlay
  (CallFunction|Widget)
  (CallFunction|AbilityInitialize))

(fn ConstructionScript)