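; Game mode that spawns enemies, respawns the player on death and shows a game clear screen.
; On BeginPlay it spawns EnemyMax behavior-tree AI enemies at randomly picked EnemySpawnArea actors.
; When the player pawn is destroyed, it spawns and possesses a new one at player start, then repoints every enemy's blackboard chase target to it.
; EnemyCheck displays the clear widget once the player's DestroyedCount equals EnemyMax.
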(event Custom|OnDestroyed_Event
  (params (DestroyedActor :type Actor%20Object%20Reference))
  (Utilities|FlowControl|Sequence
    (:then_0
      (bind _returnvalue (Game|SpawnActorfromClass "/Game/UnrealQuest5/Blueprints/BP_UQ5_Player.BP_UQ5_Player_C" (Transformation|GetActorTransform (Class|GameModeBase|FindPlayerStart)) "Undefined" 0 0))
      (Pawn|Possess (Game|GetPlayerController 0) _returnvalue)
      (Game|AssignOnDestroyed _returnvalue (delegate Custom|OnDestroyed_Event))
      (Variables|/Game/UnrealQuest5/Blueprints/BP_UQ5_Player.BP_UQ5_Player_C|SetHealth _returnvalue 1e+02)
      (Utilities|FlowControl|DoOnce false :!label _label
        (:Completed
          (bind _outactors (Actor|GetAllActorsOfClass "/Game/UnrealQuest5/Blueprints/BP_UQ5_Enemy.BP_UQ5_Enemy_C"))
          (for _array_element _outactors
            (bind _blackboardcomponent (Class|AIController|UseBlackboard (AI|GetAIController _array_element) "/Game/UnrealQuest5/AI/BB_Enemy.BB_Enemy"))
            (AI|Components|Blackboard|SetValueasObject _blackboardcomponent (Utilities|Name|MakeLiteralName "ChaseActorKey") (Game|Player|GetPlayerPawn 0)))
          (goto _label Reset))))))

(event Custom|EnemyCheck
  (bind _asbp_uq5_player (Utilities|Casting|CastToBP_UQ5_Player (Game|Player|GetPlayerPawn 0)))
  (if (== (Variables|/Game/UnrealQuest5/Blueprints/BP_UQ5_Player.BP_UQ5_Player_C|GetDestroyedCount _asbp_uq5_player) (Variables|Default|GetEnemyMax))
    (bind _returnvalue (UserInterface|CreateWidget "/Game/MyFolder/Widget/WBP_GameClear.WBP_GameClear_C"))
    (bind _output_get (Variables|Default|SetGameClear _returnvalue))
    (UserInterface|Viewport|AddtoViewport _output_get 0)))

(event Custom|InitializeEnemySpawn
  (for _index (range 0 (- (Variables|Default|GetEnemyMax) 1))
    (bind _outactors (Actor|GetAllActorsOfClass "/Game/MyFolder/MyBlueprint/EnemySpawnArea.EnemySpawnArea_C"))
    (AI|SpawnAIFromClass "/Game/UnrealQuest5/Blueprints/BP_UQ5_Enemy.BP_UQ5_Enemy_C" "/Game/UnrealQuest5/AI/BT_Enemy.BT_Enemy" (.Location (Math|Transform|BreakTransform (Transformation|GetActorTransform (.OutItem (Utilities|Array|Random _outactors))))) (.Rotation (Math|Transform|BreakTransform (Transformation|GetActorTransform (.OutItem (Utilities|Array|Random _outactors))))) false 0)))

(event EventBeginPlay
  (CallFunction|InitializeEnemySpawn)
  (Game|AssignOnDestroyed (Game|Player|GetPlayerPawn 0) (delegate Custom|OnDestroyed_Event)))

(fn ConstructionScript)